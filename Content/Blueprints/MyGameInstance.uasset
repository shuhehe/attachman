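; Game instance that drives the front-end menus and Advanced Sessions multiplayer flow.
; Show events lazily create and cache main menu, multiplayer and server list widgets before adding them to the viewport.
; Session events host, join or destroy sessions; single player and hosting both open ThirdPersonExampleMap as a listen server.
; FindSession is an empty event, with its search-and-join logic left disconnected, and StartSinglePlayer sets IsSinglePlayer to false.
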(event Custom|FindSession
  ;[1 1 1] FindSession
)

(event Custom|JoinSession
  (params (Session :type Blueprint%20Session%20Result%20Structure))
  ;[1 1 1] JoinSession
  (Widget|RemovefromParent (Variables|Default|GetBPWServerListRef))
  (|JoinSession (Game|GetPlayerController 0) Session
    (:OnFailure
      (Development|PrintString "Failed To Join Session!!!" true true "(R=1.000000,G=0.000000,B=0.000000,A=1.000000)" 4.0))))

(event Custom|DestroySessionCaller
  (params (PlayerController :type Player%20Controller%20Object%20Reference))
  ;[1 1 1] DestroySession
  (Variables|Default|SetIsSinglePlayer? false)
  (|DestroySession PlayerController))

(event Custom|CreateSession
  (bind _returnvalue (Game|GetPlayerController 0))
  ;[1 1 1] Creat Session
  (|AdvancedSession 0 (Game|GetPlayerController 0) 100 0 false true false true true false false false true
    (:OnSuccess
      (Game|OpenLevel(byName) "ThirdPersonExampleMap" true "listen")
      (Input|SetInputModeGameOnly _returnvalue)
      (Variables|/Script/Engine.PlayerController|SetbShowMouseCursor _returnvalue false))
    (:OnFailure
      (Development|PrintString "Host Game Failed!!!!" true true "(R=1.000000,G=0.000000,B=0.000000,A=1.000000)" 4.0))))

(event Custom|StartSinglePlayer
  (bind _returnvalue (Game|GetPlayerController 0))
  ;[1 1 1] SinglePlayer
  (Variables|Default|SetIsSinglePlayer? false)
  (Game|OpenLevel(byName) "ThirdPersonExampleMap" true "listen")
  (Input|SetInputModeGameOnly _returnvalue)
  (Variables|/Script/Engine.PlayerController|SetbShowMouseCursor _returnvalue false))

(event Custom|ShowMainMenu
  (bind _returnvalue (Game|GetPlayerController 0))
  ;[1 1 1] Show MainMenu
  (Utilities|IsValid (Variables|Default|GetBPWMainMenuRef)
    (:Is%20Valid
      _)
    (:Is%20Not%20Valid
      (bind _returnvalue_2 (UserInterface|CreateWidget "/Game/UMG/WBP_MainMenu.WBP_MainMenu_C" _returnvalue))
      (Variables|Default|SetBPWMainMenuRef _returnvalue_2)))
  (UserInterface|Viewport|AddtoViewport (Variables|Default|GetBPWMainMenuRef) 0)
  (Input|SetInputModeUIOnly _returnvalue (Variables|Default|GetBPWMainMenuRef) "DoNotLock")
  (Variables|/Script/Engine.PlayerController|SetbShowMouseCursor _returnvalue true))

(event Custom|ShowServerList
  ;[1 1 1] ShowServerList
  (Utilities|IsValid (Variables|Default|GetBPWServerListRef)
    (:Is%20Valid
      _)
    (:Is%20Not%20Valid
      (bind _returnvalue (UserInterface|CreateWidget "/Game/UMG/WBP_ServerList.WBP_ServerList_C" (Game|GetPlayerController 0)))
      (Variables|Default|SetBPWServerListRef _returnvalue)))
  (UserInterface|Viewport|AddtoViewport (Variables|Default|GetBPWServerListRef) 0))

(event Custom|ShowMultiplayerMenu
  ;[1 1 1] ShowMultiplayerMenu
  (Utilities|IsValid (Variables|Default|GetBPWMultiplayerMenuRef)
    (:Is%20Valid
      _)
    (:Is%20Not%20Valid
      (bind _returnvalue (UserInterface|CreateWidget "/Game/UMG/WBP_Multiplayer.WBP_Multiplayer_C" (Game|GetPlayerController 0)))
      (Variables|Default|SetBPWMultiplayerMenuRef _returnvalue)))
  (UserInterface|Viewport|AddtoViewport (Variables|Default|GetBPWMultiplayerMenuRef) 0))