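; BP_GS_MP_TPSBasic is a multiplayer third-person Blueprint, apparently a Game State by its name, that handles restarting the example map through server travel.
; Its Server_TravelToMap event checks the current level name and, on ThirdPersonExampleMap, runs a servertravel console command back to that same map.
; The two nested fallback branches repeat the identical check and command, so any other level triggers no travel.
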(event Custom|Server_TravelToMap
  (bind _returnvalue (Game|GetCurrentLevelName true))
  (if (Utilities|Name|Equal(Name) (Utilities|String|StringToName _returnvalue) "ThirdPersonExampleMap")
    (Development|ExecuteConsoleCommand "servertravel ThirdPersonExampleMap" 0)
    (elif (Utilities|Name|Equal(Name) (Utilities|String|StringToName _returnvalue) "ThirdPersonExampleMap")
      (Development|ExecuteConsoleCommand "servertravel ThirdPersonExampleMap" 0)
      (elif (Utilities|Name|Equal(Name) (Utilities|String|StringToName _returnvalue) "ThirdPersonExampleMap")
        (Development|ExecuteConsoleCommand "servertravel ThirdPersonExampleMap" 0)))))

(fn ConstructionScript)