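; Main menu game mode that spawns and possesses player characters at random Player Start points.
; Shortly after BeginPlay, or on RefreshSpawnPoints, the authority rebuilds an array of all PlayerStart actors.
; Server_RespawnPlayer draws from that array to spawn a ThirdPersonCharacter, adjusting for collisions but always spawning, then has the given controller possess it.
; Despite the graph comment mentioning team spawn arrays, selection ignores teams.
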(event Custom|Server_RespawnPlayer
  (params (PlayerController :type Player%20Controller%20Object%20Reference))
  (bind _spawnpoint (Variables|Default|GetSpawnPoint))
  (bind _returnvalue (Utilities|Array|Length _spawnpoint))
  (bind _returnvalue_2 (- _returnvalue 1))
  (bind _returnvalue_3 (Math|Random|RandomIntegerinRange 0 _returnvalue_2))
  (bind _output (Utilities|Array|Get(acopy) _spawnpoint _returnvalue_3))
  (bind _returnvalue_4 (Transformation|GetActorTransform _output))
  ;[1 1 1] Server Respawn Player Selects A Random Spawn Location Based On Team From Team Spawn Points Arrays
  (Utilities|IsValid PlayerController
    (:Is%20Valid
      (bind _returnvalue_5 (Game|SpawnActorfromClass "/Game/ThirdPersonCPP/Blueprints/ThirdPersonCharacter.ThirdPersonCharacter_C" (Math|Transform|MakeTransform (.location _returnvalue_4) (.rotation _returnvalue_4) "1,1,1") "AdjustIfPossibleButAlwaysSpawn" 0 0))
      (Utilities|IsValid _returnvalue_5
        (:Is%20Valid
          (Pawn|Possess PlayerController _returnvalue_5))))))

(event Custom|RefreshSpawnPoints
  ;[1 1 1] Event Begin Play Build Array Of Spawn Points
  (Networking|SwitchHasAuthority
    (:Authority
      (Utilities|Array|Clear (Variables|Default|GetSpawnPoint))
      (bind _outactors (Actor|GetAllActorsOfClass "/Script/Engine.PlayerStart"))
      (for _array_element _outactors
        (Utilities|Array|Add (Variables|Default|GetSpawnPoint) _array_element)))))

(event EventBeginPlay
  ;[1 1 1] Event Begin Play Build Array Of Spawn Points
  (Utilities|FlowControl|Delay 0.5)
  (Networking|SwitchHasAuthority
    (:Authority
      (Utilities|Array|Clear (Variables|Default|GetSpawnPoint))
      (bind _outactors (Actor|GetAllActorsOfClass "/Script/Engine.PlayerStart"))
      (for _array_element _outactors
        (Utilities|Array|Add (Variables|Default|GetSpawnPoint) _array_element)))))

(fn ConstructionScript)